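; Player-controllable tank pawn Blueprint that handles third-person camera aiming and forward/backward movement input.
; Aim axes split the orbit: azimuth yaws a gimbal component, while zenith pitches the third-person spring arm.
; The movement axis feeds AddMovementInput along the Tank component's forward vector, independent of the aim rotation.
; All three axes scale by frame delta time and a fixed rate; the construction script is empty.
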(event `InputAxis|AimAzimuth`
  (params (AxisValue :type "Float (single-precision)"))
  ;[1 1 1] Camera Input Bindings
  (`SceneComponent.K2_AddLocalRotation` (`self.Azimuth Gimbal`) (`KismetMathLibrary.MakeRotator` 0.0 0.0 (* AxisValue (`GameplayStatics.GetWorldDeltaSeconds`) 100.0)) false false))

(event `InputAxis|AimZenith`
  (params (AxisValue :type "Float (single-precision)"))
  ;[1 1 1] Camera Input Bindings
  (`SceneComponent.K2_AddLocalRotation` (`self.3rdPersonSpringArm`) (`KismetMathLibrary.MakeRotator` 0.0 (* AxisValue (`GameplayStatics.GetWorldDeltaSeconds`) 100.0)) false false))

(event `InputAxis|StraightMovement`
  (params (AxisValue :type "Float (single-precision)"))
  (`self.AddMovementInput` (`SceneComponent.GetForwardVector` (`self.Tank`)) (* AxisValue (`GameplayStatics.GetWorldDeltaSeconds`) 100.0)))

(fn `UserConstructionScript`)